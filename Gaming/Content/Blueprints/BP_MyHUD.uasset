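; HUD Blueprint that sets up the main on-screen HUD and manages showing and hiding the inventory screen.
; On BeginPlay it adds a MainHUD widget to the viewport and creates an Inventory widget, stored for later use.
; ToggleInv shows the inventory with UI-only input and a mouse cursor, or restores game-only input and hides the cursor.
; Hiding calls RemoveAllWidgets, so MainHUD is removed too and is not re-added here.
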(event EventBeginPlay
  (bind _returnvalue (UserInterface|CreateWidget "/Game/Widgets/MainHUD.MainHUD_C" (Game|GetPlayerController 0)))
  (UserInterface|Viewport|AddtoViewport _returnvalue 0)
  (bind _returnvalue_2 (UserInterface|CreateWidget "/Game/Widgets/Inventory.Inventory_C"))
  (Variables|Default|SetWidgetInv _returnvalue_2))

(event Collision|EventActorBeginOverlap
  (params (OtherActor :type Actor%20Object%20Reference)))

(event EventTick
  (params (DeltaSeconds :type Float%20%28single-precision%29)))

(fn ConstructionScript)

(fn ToggleInv
  (params (Show :type Boolean))
  (bind _returnvalue (Game|GetPlayerController 0))
  (bind _widgetinv (Variables|Default|GetWidgetInv))
  (if Show
    (UserInterface|Viewport|AddtoViewport _widgetinv 0)
    (Input|SetInputModeUIOnly _returnvalue _widgetinv "DoNotLock")
    (Variables|/Script/Engine.PlayerController|SetbShowMouseCursor _returnvalue true)
    (else
      (Viewport|RemoveAllWidgets)
      (Input|SetInputModeGameOnly _returnvalue)
      (Variables|/Script/Engine.PlayerController|SetbShowMouseCursor _returnvalue false))))