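; BP_Hero is the player hero Blueprint that picks up items on overlap and opens the inventory UI.
; Overlapped Item actors are added to Inventory while it is below InventorySlots, then hidden with collision disabled rather than destroyed.
; BeginPlay caches BP_MyHUD from the first player controller for the ShowInventory input.
; That input runs a FlipFlop, but both branches call ToggleInv with true.
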(event EventBeginPlay
  (bind _asbp_my_hud (Utilities|Casting|CastToBP_MyHUD (HUD|GetHUD (Game|GetPlayerController 0))))
  (Variables|Default|SetHUD _asbp_my_hud))

(event Collision|EventActorBeginOverlap
  (params (OtherActor :type Actor%20Object%20Reference))
  (bind _inventory (Variables|Default|GetInventory))
  (bind _asitem (Utilities|Casting|CastToItem OtherActor))
  (if (not (<= (Variables|Default|GetInventorySlots) (Math|Conversions|ToFloat(Integer) (Utilities|Array|Length _inventory))))
    (Utilities|Array|Add _inventory _asitem)
    (Rendering|SetActorHiddenInGame _asitem true)
    (Collision|SetActorEnableCollision _asitem false)))

(event EventTick
  (params (DeltaSeconds :type Float%20%28single-precision%29)))

(event Input|ActionEvents|InputActionShowInventory
  (params (Key :type Key%20Structure :default "None"))
  (bind _hud (Variables|Default|GetHUD))
  (:Pressed
    (Utilities|FlowControl|FlipFlop
      (:A
        (Default|ToggleInv _hud true))
      (:B
        (Default|ToggleInv _hud true)))))

(fn ConstructionScript)